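; BP_WardrobeDoor is an interactable wardrobe door that swings open and closed by 90 degrees of yaw.
; Interact, gated by CanPressE and CanInteract, toggles Opened and plays the TL_Rotate timeline from start or in reverse.
; The timeline lerps mesh yaw from the rotation cached at BeginPlay.
; A short Delay on the timeline's update re-enables interaction, independently of the swing finishing.
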(event `self.ReceiveBeginPlay`
  (set `self.StartingRotation` (`SceneComponent.RelativeRotation` (`self.StaticMesh`))))

(event `/Game/Framework/bpi_Interaction.Interact`
  (bind (_startingrotation_roll _startingrotation_pitch _startingrotation_yaw) (`KismetMathLibrary.BreakRotator` (`self.StartingRotation`)))
  (if (`self.CanPressE`)
    (if (`self.CanInteract`)
      (set `self.CanInteract` false)
      (if (`self.Opened`)
        (set `self.Opened` false)
        (bind (_direction _alpha) (`Timeline|TL_Rotate` :!via `Reverse` :!label _label)
          (:`Update`
            (`SceneComponent.K2_SetRelativeRotation` (`self.StaticMesh`) (`KismetMathLibrary.MakeRotator` _startingrotation_roll _startingrotation_pitch (`KismetMathLibrary.Lerp` _startingrotation_yaw (- _startingrotation_yaw 90.0) _alpha)) false false)
            (`KismetSystemLibrary.Delay` 0.2)
            (set `self.CanInteract` true)))
        (else
          (set `self.Opened` true)
          (goto _label :!via `PlayFromStart`))))))

(fn `UserConstructionScript`
  (`parent.UserConstructionScript`))