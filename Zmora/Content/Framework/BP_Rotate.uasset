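; BP_Rotate is an actor that spins itself around its local yaw axis for a short timed window after play starts.
; BeginPlay uses two delays to switch an active flag on, then off again.
; While the flag is set, Tick adds a negative yaw offset scaled by frame time and a Rotation variable.
; A sphere overlap event repeats the rotation call with a zero multiplier, so it has no visible effect.
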(event `self.ReceiveBeginPlay`
  (`KismetSystemLibrary.Delay` 1.0)
  (set `self.isactive` true)
  (`KismetSystemLibrary.Delay` 1.0)
  (set `self.isactive` false))

(event `self.ReceiveTick`
  (params (DeltaSeconds :type "Float (single-precision)"))
  (if (`self.isactive`)
    (`self.K2_AddActorLocalRotation` (`KismetMathLibrary.MakeRotator` 0.0 0.0 (* (* DeltaSeconds (`self.Rotation`)) -2.0)))))

(event `self.Sphere.OnComponentBeginOverlap`
  (params (OverlappedComponent :type "PrimitiveComponent Object Reference") (OtherActor :type "Actor Object Reference") (OtherComp :type "PrimitiveComponent Object Reference") (OtherBodyIndex :type Integer) (bFromSweep :type Boolean) (SweepResult :type "HitResult Structure (by ref)"))
  (if (`self.isactive`)
    (`self.K2_AddActorLocalRotation` (`KismetMathLibrary.MakeRotator` 0.0 0.0 (* (* 0.0 (`self.Rotation`)) -2.0)))))

(fn `UserConstructionScript`)